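; Dog anatomy actor for a VR game, with static mesh components for bones, internal organs and skin.
; On BeginPlay it caches the player's VRPawn, stopping if the cast fails, then gathers all static mesh components and removes the skin and named organs to leave a bone list.
; It also groups named front-leg bone components into a FrontLegs array.
; The graphs only perform this setup, with no Tick, overlap or construction logic.
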(event EventBeginPlay
  (bind _asvrpawn (Utilities|Casting|CastToVRPawn (Game|Player|GetPlayerPawn 0)))
  (Variables|Default|SetVRPawn _asvrpawn)
  (bind _output_get (Variables|Default|SetBone_StaticMeshes (Actor|GetComponentsByClass "/Script/Engine.StaticMeshComponent")))
  (Utilities|Array|RemoveItem _output_get (Variables|Default|GetEsophagus))
  (Utilities|Array|RemoveItem _output_get (Variables|Default|GetHeart))
  (Utilities|Array|RemoveItem _output_get (Variables|Default|GetLungs))
  (Utilities|Array|RemoveItem _output_get (Variables|Default|GetSkin))
  (Utilities|Array|RemoveItem _output_get (Variables|Default|GetBladder))
  (Utilities|Array|RemoveItem _output_get (Variables|Default|GetDuodenum))
  (Utilities|Array|RemoveItem _output_get (Variables|Default|GetKidney))
  (Utilities|Array|RemoveItem _output_get (Variables|Default|GetSpleen))
  (Utilities|Array|RemoveItem _output_get (Variables|Default|GetStomach))
  (Variables|Default|SetFront_Legs (Utilities|Array|MakeArray (Variables|Default|GetInfraspinous_Fossa_Left) (Variables|Default|GetAcromion_Right) (Variables|Default|GetC_Base_L) (Variables|Default|GetC_Base_R) (Variables|Default|GetGreater_Tubercle) (Variables|Default|GetHead_of_Humerus_Left) (Variables|Default|GetHead_of_Humerus_Right) (Variables|Default|GetHumeral_Shaft) (Variables|Default|GetAcromion_Left) (Variables|Default|GetInfraspinous_Fossa_Right) (Variables|Default|GetSupraglenoid_Tubercle_Left) (Variables|Default|GetSupraglenoid_Tubercle_Right) (Variables|Default|GetSupraspinous_Fossa_Left) (Variables|Default|GetSupraspinous_Fossa_Right) (Variables|Default|GetTricipital_Line_Left) (Variables|Default|GetTricipital_Line_Right) (Variables|Default|GetBody_of_Ulna) (Variables|Default|GetD_Base) (Variables|Default|GetHead_of_Radius) (Variables|Default|GetOlecranon) (Variables|Default|GetOlecranon_Tuber) (Variables|Default|GetStyloid_Process_of_Radius) (Variables|Default|GetStyloid_process_of_Ulna) (Variables|Default|GetBody_of_Radius) (Variables|Default|GetE_17) (Variables|Default|GetE_10) (Variables|Default|GetE_11) (Variables|Default|GetE_12) (Variables|Default|GetE_16) (Variables|Default|GetE_Base) (Variables|Default|GetE_18) (Variables|Default|GetE_19) (Variables|Default|GetE_20) (Variables|Default|GetE_21))))

(event Collision|EventActorBeginOverlap
  (params (OtherActor :type Actor%20Object%20Reference)))

(event EventTick
  (params (DeltaSeconds :type Float%20%28single-precision%29)))

(fn ConstructionScript)